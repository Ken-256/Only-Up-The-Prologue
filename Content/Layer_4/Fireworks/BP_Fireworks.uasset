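; BP_Fireworks is a proximity-triggered fireworks actor that runs while the third-person character is inside its Box volume.
; Box overlap begin, filtered by a cast to BP_ThirdPersonCharacter, plays the Fireworks component from the start, activates the NSFireworks effect and sets IsPlaying.
; Overlap end stops both components and clears the flag.
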(event `self.ReceiveActorBeginOverlap`
  (params (OtherActor :type "Actor Object Reference")))

(event `self.Box.OnComponentBeginOverlap`
  (params (OverlappedComponent :type "PrimitiveComponent Object Reference") (OtherActor :type "Actor Object Reference") (OtherComp :type "PrimitiveComponent Object Reference") (OtherBodyIndex :type Integer) (bFromSweep :type Boolean) (SweepResult :type "HitResult Structure (by ref)"))
  (cast `/Game/ThirdPerson/Blueprints/BP_ThirdPersonCharacter` OtherActor)
  (if true
    (`AudioComponent.Play` (`self.Fireworks`) 0.0)
    (`ActorComponent.Activate` (`self.NS_Fireworks`) false)
    (set `self.IsPlaying` true)))

(event `self.Box.OnComponentEndOverlap`
  (params (OverlappedComponent :type "PrimitiveComponent Object Reference") (OtherActor :type "Actor Object Reference") (OtherComp :type "PrimitiveComponent Object Reference") (OtherBodyIndex :type Integer))
  (cast `/Game/ThirdPerson/Blueprints/BP_ThirdPersonCharacter` OtherActor)
  (if true
    (`AudioComponent.Stop` (`self.Fireworks`))
    (`ActorComponent.Deactivate` (`self.NS_Fireworks`))
    (set `self.IsPlaying` false)))

(fn `UserConstructionScript`)